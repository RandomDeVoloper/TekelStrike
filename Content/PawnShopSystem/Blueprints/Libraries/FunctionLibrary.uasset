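; Shared function library for the pawn shop system, handling wallet and bank money, the item inventory, and small helpers for HUD lookup and mesh spinning.
; Money and inventory state live in BP_GameInstance; transfers skip balance checks, and only deposit-all and withdraw-all create W_TransactionButton log entries.
; Inventory functions search linearly by item name, stacking quantities and overwriting prices on add, and removing one unit at a time.
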(fn GetGameInstance
  (bind _asbp_game_instance (Utilities|Casting|CastToBP_GameInstance (Game|GetGameInstance)))
  (return _asbp_game_instance))

(fn GetHUD
  (bind _returnvalue (Actor|GetActorOfClass 0 "/Game/PawnShopSystem/Blueprints/BP_HUD.BP_HUD_C"))
  (return _returnvalue))

(fn DepositFunds
  (params (Amount :type Integer))
  (bind _return_value (CallFunction|GetGameInstance))
  (Variables|/Game/PawnShopSystem/Blueprints/Classes/BP_GameInstance.BP_GameInstance_C|SetWallet _return_value (- (Variables|/Game/PawnShopSystem/Blueprints/Classes/BP_GameInstance.BP_GameInstance_C|GetWallet _return_value) Amount))
  (Variables|/Game/PawnShopSystem/Blueprints/Classes/BP_GameInstance.BP_GameInstance_C|SetBank _return_value (+ (Variables|/Game/PawnShopSystem/Blueprints/Classes/BP_GameInstance.BP_GameInstance_C|GetBank _return_value) Amount))
  (return))

(fn WithdrawlFunds
  (params (Amount :type Integer))
  (bind _return_value (CallFunction|GetGameInstance))
  (Variables|/Game/PawnShopSystem/Blueprints/Classes/BP_GameInstance.BP_GameInstance_C|SetBank _return_value (- (Variables|/Game/PawnShopSystem/Blueprints/Classes/BP_GameInstance.BP_GameInstance_C|GetBank _return_value) Amount))
  (Variables|/Game/PawnShopSystem/Blueprints/Classes/BP_GameInstance.BP_GameInstance_C|SetWallet _return_value (+ (Variables|/Game/PawnShopSystem/Blueprints/Classes/BP_GameInstance.BP_GameInstance_C|GetWallet _return_value) Amount)))

(fn MakeTransactionLog
  (params (Transaction%20Name :type Text) (Transaction%20Amount :type Integer))
  (bind _returnvalue (UserInterface|CreateWidget "/Game/PawnShopSystem/Widgets/W_TransactionButton.W_TransactionButton_C"))
  (Default|SetTransaction _returnvalue Transaction%20Name Transaction%20Amount)
  (return))

(fn DepositAllFunds
  (bind _return_value (CallFunction|GetGameInstance))
  (Variables|/Game/PawnShopSystem/Blueprints/Classes/BP_GameInstance.BP_GameInstance_C|SetBank _return_value (+ (Variables|/Game/PawnShopSystem/Blueprints/Classes/BP_GameInstance.BP_GameInstance_C|GetWallet _return_value) (Variables|/Game/PawnShopSystem/Blueprints/Classes/BP_GameInstance.BP_GameInstance_C|GetBank _return_value)))
  (CallFunction|MakeTransactionLog "Deposit" (Variables|/Game/PawnShopSystem/Blueprints/Classes/BP_GameInstance.BP_GameInstance_C|GetWallet _return_value))
  (Variables|/Game/PawnShopSystem/Blueprints/Classes/BP_GameInstance.BP_GameInstance_C|SetWallet _return_value 0)
  (return))

(fn WithdrawlAllFunds
  (bind _return_value (CallFunction|GetGameInstance))
  (Variables|/Game/PawnShopSystem/Blueprints/Classes/BP_GameInstance.BP_GameInstance_C|SetWallet _return_value (+ (Variables|/Game/PawnShopSystem/Blueprints/Classes/BP_GameInstance.BP_GameInstance_C|GetWallet _return_value) (Variables|/Game/PawnShopSystem/Blueprints/Classes/BP_GameInstance.BP_GameInstance_C|GetBank _return_value)))
  (CallFunction|MakeTransactionLog "Withdrawl" (- 0 (Variables|/Game/PawnShopSystem/Blueprints/Classes/BP_GameInstance.BP_GameInstance_C|GetBank _return_value)))
  (Variables|/Game/PawnShopSystem/Blueprints/Classes/BP_GameInstance.BP_GameInstance_C|SetBank _return_value 0)
  (return))

(fn AddMeshRotation
  (params (Delta%20Seconds :type Float%20%28double-precision%29) (Static%20Mesh :type Scene%20Component%20Object%20Reference) (Rotation%20Speed :type Float%20%28double-precision%29))
  (Transformation|AddLocalRotation Static%20Mesh (* (Math|Rotator|MakeRotator 0.0 0.0 Rotation%20Speed) Delta%20Seconds) false false))

(fn AddItemtoInventory
  (params (Item%20Name :type Text%20%28by%20ref%29) (Quantity :type Integer) (Retail%20Price :type Integer) (Minimal%20Offer :type Integer))
  (bind _return_value (CallFunction|GetGameInstance))
  (bind _s_inventory (Variables|/Game/PawnShopSystem/Blueprints/Classes/BP_GameInstance.BP_GameInstance_C|GetS_Inventory _return_value))
  (bind (_array_element _array_index) (Utilities|Array|ForEachLoopwithBreak _s_inventory :!label _label)
    (:LoopBody
      (if (Utilities|Enum|Equal(Enum) (.ItemName (Utilities|Struct|BreakS_Inventory _array_element)) Item%20Name)
        (LocalVariables|SetContains true)
        (goto _label Break)))
    (:Completed
      (if (LocalVariables|GetContains)
        (Utilities|Array|SetArrayElem _s_inventory _array_index (Utilities|Struct|MakeS_Inventory (.ItemName (Utilities|Struct|BreakS_Inventory _array_element)) (+ (.Quantity (Utilities|Struct|BreakS_Inventory _array_element)) Quantity) Retail%20Price Minimal%20Offer))
        (else
          (Utilities|Array|Add _s_inventory (Utilities|Struct|MakeS_Inventory Item%20Name Quantity Retail%20Price Minimal%20Offer))))
      (return))))

(fn RemovefromInventory
  (params (Item%20Name :type Text%20%28by%20ref%29))
  (bind _return_value (CallFunction|GetGameInstance))
  (bind _s_inventory (Variables|/Game/PawnShopSystem/Blueprints/Classes/BP_GameInstance.BP_GameInstance_C|GetS_Inventory _return_value))
  (bind (_array_element _array_index) (Utilities|Array|ForEachLoopwithBreak _s_inventory :!label _label)
    (:LoopBody
      (if (Utilities|Enum|Equal(Enum) (.ItemName (Utilities|Struct|BreakS_Inventory _array_element)) Item%20Name)
        (LocalVariables|SetContains true)
        (goto _label Break)))
    (:Completed
      (if (LocalVariables|GetContains)
        (if (not (== (.Quantity (Utilities|Struct|BreakS_Inventory _array_element)) 1))
          (Utilities|Array|SetArrayElem _s_inventory _array_index (Utilities|Struct|MakeS_Inventory Item%20Name (- (.Quantity (Utilities|Struct|BreakS_Inventory _array_element)) 1) (.RetailPrice (Utilities|Struct|BreakS_Inventory _array_element)) (.MinimalOffer (Utilities|Struct|BreakS_Inventory _array_element))))
          (elif (<= (- (.Quantity (Utilities|Struct|BreakS_Inventory _array_element)) 1) 0)
            (Development|PrintString 0 "eksidesin looo nasıl yaptın")
            (Utilities|Array|RemoveItem _s_inventory _array_element)))))))

(fn CheckItemQuantity
  (params (Item%20Name :type Text%20%28by%20ref%29))
  (bind _array_element (Utilities|Array|ForEachLoopwithBreak (Variables|/Game/PawnShopSystem/Blueprints/Classes/BP_GameInstance.BP_GameInstance_C|GetS_Inventory (CallFunction|GetGameInstance)) :!label _label)
    (:LoopBody
      (if (Utilities|Enum|Equal(Enum) (.ItemName (Utilities|Struct|BreakS_Inventory _array_element)) Item%20Name)
        (LocalVariables|SetContains true)
        (goto _label Break)))
    (:Completed
      (if (LocalVariables|GetContains)
        (return (.Quantity (Utilities|Struct|BreakS_Inventory _array_element)))))))