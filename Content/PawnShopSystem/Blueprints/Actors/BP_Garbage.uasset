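; BP_Garbage is a garbage item that the player can pick up into inventory or that reacts to impacts.
; Box overlap shows W_Interact and gates the Interact input, which adds the item and destroys the actor.
; The first mesh hit randomly triggers either a police warning popup or a radial impulse with explosion sounds, decal and camera shake.
; Hitting BP_A/B/C1 also enables their mesh physics; disconnected Molotov logic remains.
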(event OnComponentBeginOverlap(Box)
  (params (OverlappedComponent :type Primitive%20Component%20Object%20Reference) (OtherActor :type Actor%20Object%20Reference) (OtherComp :type Primitive%20Component%20Object%20Reference) (OtherBodyIndex :type Integer) (bFromSweep :type Boolean) (SweepResult :type Hit%20Result%20Structure%20%28by%20ref%29))
  ;[0 0 0] Player Interaction
  (if (== OtherActor (Game|GetPlayerCharacter 0))
    (Input|EnableInput (Game|GetPlayerController 0))
    (bind _returnvalue (UserInterface|CreateWidget "/Game/PawnShopSystem/Widgets/W_Interact.W_Interact_C" 0 (Variables|Default|GetInteraction%20Name)))
    (UserInterface|Viewport|AddtoViewport _returnvalue 0)
    (Utilities|FlowControl|Gate true) ; enters at Open
  ))

(event OnComponentEndOverlap(Box)
  (params (OverlappedComponent :type Primitive%20Component%20Object%20Reference) (OtherActor :type Actor%20Object%20Reference) (OtherComp :type Primitive%20Component%20Object%20Reference) (OtherBodyIndex :type Integer))
  ;[0 0 0] Player Interaction
  (if (== (Game|GetPlayerCharacter 0) OtherActor)
    (Input|DisableInput (Game|GetPlayerController 0))
    (Widget|RemovefromParent (stale OnComponentBeginOverlap(Box) _returnvalue))
    (Utilities|FlowControl|Gate true) ; enters at Close
  ))

(event OnComponentBeginOverlap(StaticMesh)
  (params (OverlappedComponent :type Primitive%20Component%20Object%20Reference) (OtherActor :type Actor%20Object%20Reference) (OtherComp :type Primitive%20Component%20Object%20Reference) (OtherBodyIndex :type Integer) (bFromSweep :type Boolean) (SweepResult :type Hit%20Result%20Structure%20%28by%20ref%29))
  ;[0 0 0] Player Interaction
)

(event OnComponentHit(StaticMesh)
  (params (HitComponent :type Primitive%20Component%20Object%20Reference) (OtherActor :type Actor%20Object%20Reference) (OtherComp :type Primitive%20Component%20Object%20Reference) (NormalImpulse :type Vector :default "0, 0, 0") (Hit :type Hit%20Result%20Structure%20%28by%20ref%29))
  (bind (_x _y) (Math|Vector|BreakVector (.location Hit)))
  (Utilities|FlowControl|Sequence
    (:then_0
      ;[0.15 0.15 0.15 0.5] PATLAMA OLASILIĞI
      (Utilities|FlowControl|DoOnce false
        (:Completed
          ;[0.15 0.15 0.15 0.5] POLİS ANONSU Kontrolü
          (if (>= (Math|Random|RandomIntegerinRange 0 10) 8)
            (Utilities|FlowControl|DoOnce false
              (:Completed
                ;[0.15 0.15 0.15 0.5] ULAN GERİZEKALI NEREYE ATIYOSUN
                (Audio|PlaySound2D "/Game/Developers/Ulan-Gerizekalı-Nereye-Atıyorsun-Ses-Efekti-_uCWYe0-FLS8_.Ulan-Gerizekalı-Nereye-Atıyorsun-Ses-Efekti-_uCWYe0-FLS8_" 2.0 1.0 0.0 0 0)
                ;[0.15 0.15 0.15 0.5] polis widgetı
                (bind _returnvalue (UserInterface|CreateWidget "/Game/Widgets/WBP_Polis.WBP_Polis_C" (Game|GetPlayerController 0)))
                (bind _output_get (Variables|Default|SetWBP_PolicREF _returnvalue))
                (UserInterface|Viewport|AddtoViewport _output_get 0)
                (UserInterface|Animation|PlayAnimation _output_get (Variables|/Game/Widgets/WBP_Polis.WBP_Polis_C|GetPopUpAnim _output_get) 0.0 2 "Forward" 0.7 false)
                (Utilities|FlowControl|Delay 2.0)
                (Widget|RemovefromParent _output_get)))
            (else
              (Class|RadialForceComponent|FireImpulse (Variables|Default|GetRadialForce))
              ;[0.15 0.15 0.15 0.5] BOMBA PATLAMA
              (Audio|PlaySoundatLocation "/Game/PawnShopSystem/Blueprints/Actors/garbageExplode.garbageExplode" (.location Hit) "0, 0, 0" 0.01 1.0 0.0 0 0 0 0 :!label _label)
              (Audio|PlaySoundatLocation 0 (.location Hit) "0, 0, 0" 1.0 1.0 0.0 0 0 0 0)
              (Audio|PlaySoundatLocation "/Game/Assets/Sound/MolotofFireLand.MolotofFireLand" (.location Hit) (Math|Conversions|RotationFromXVector (.location Hit)) 1.0 1.0 0.0 0 0 0 0)
              (Rendering|Decal|SpawnDecalatLocation "/Game/Assets/Ickiler/M_Decal.M_Decal" "75.000000,75.000000,75.000000" (Math|Vector|MakeVector _x _y 0.0) "-90.000000,0.000000,0.000000" 35.0)
              (Camera|PlayWorldCameraShake "/Game/Blueprints/CameraShake/BP_CamSHakee.BP_CamSHakee_C" (.location Hit) 0.0 1.25e+04)
              (Utilities|FlowControl|Delay 2.0))))))
    (:then_1
      (bind _asbp_a (Utilities|Casting|CastToBP_A OtherActor))
      (Class|RadialForceComponent|FireImpulse (Variables|Default|GetRadialForce))
      (Physics|SetSimulatePhysics (Variables|/Script/Engine.Character|GetMesh _asbp_a) true)
      (Utilities|FlowControl|Delay 1.0)
      (goto _label))
    (:then_2
      (bind _asbp_b (Utilities|Casting|CastToBP_B OtherActor))
      (Class|RadialForceComponent|FireImpulse (Variables|Default|GetRadialForce))
      (Physics|SetSimulatePhysics (Variables|/Script/Engine.Character|GetMesh _asbp_b) true)
      (Utilities|FlowControl|Delay 1.0)
      (goto _label))
    (:then_3
      (bind _asbp_c1 (Utilities|Casting|CastToBP_C1 OtherActor))
      (Class|RadialForceComponent|FireImpulse (Variables|Default|GetRadialForce))
      (Physics|SetSimulatePhysics (Variables|/Script/Engine.Character|GetMesh _asbp_c1) true)
      (Utilities|FlowControl|Delay 1.0)
      (goto _label))))

(event OnComponentSleep(StaticMesh)
  (params (SleepingComponent :type Primitive%20Component%20Object%20Reference) (BoneName :type Name :default "None"))
  ;[0.15 0.15 0.15 0.5] Comment
)

(event Custom|PolisAnons
  ;[0.15 0.15 0.15 0.5] POLİS
  ;;[0.15 0.15 0.15 0.5] ULAN GERİZEKALI NEREYE ATIYOSUN
  (Audio|PlaySound2D "/Game/Developers/Ulan-Gerizekalı-Nereye-Atıyorsun-Ses-Efekti-_uCWYe0-FLS8_.Ulan-Gerizekalı-Nereye-Atıyorsun-Ses-Efekti-_uCWYe0-FLS8_" 2.0 1.0 0.0 0 0)
  (Development|PrintString "ashadhdshdsHello")
  (Utilities|FlowControl|DoOnce false :!label _label
    (:Completed
      (Utilities|FlowControl|Delay 0.04)
      (bind _returnvalue (UserInterface|CreateWidget "/Game/Widgets/WBP_Polis.WBP_Polis_C" (Game|GetPlayerController 0)))
      (bind _output_get (Variables|Default|SetWBP_PolicREF _returnvalue))
      (UserInterface|Viewport|AddtoViewport _output_get 0)
      (UserInterface|Animation|PlayAnimation _output_get (Variables|/Game/Widgets/WBP_Polis.WBP_Polis_C|GetPopUpAnim _output_get) 0.0 2 "Forward" 0.7 false)
      (Utilities|FlowControl|Delay 2.0)
      (Widget|RemovefromParent _output_get)
      (goto _label Reset))))

(event Input|ActionEvents|InputActionInteract
  (params (Key :type Key%20Structure :default "None"))
  ;[0 0 0] Player Interaction
  (:Pressed
    (Utilities|FlowControl|Gate true
      (:Exit
        ;[0 0 0] Add item to player inventory and destroy actor after pickup
        (CallFunction|AddItemtoInventory (Variables|Default|GetItem%20Name) (Variables|Default|GetQuantity) (Variables|Default|GetRetail%20Price) (Variables|Default|GetMinimal%20Offer))
        (Actor|DestroyActor)))))

(fn ConstructionScript)

(fn BombaPatlama
  (params (InputPin :type Vector))
  (bind (_x _y) (Math|Vector|BreakVector InputPin))
  (bind (_x_2 _y_2) (Math|Vector|BreakVector InputPin))
  (Utilities|FlowControl|DoOnce false
    (:Completed
      (Effects|SpawnEmitteratLocation "/Game/StarterContent/Particles/P_Explosion.P_Explosion" InputPin "0, 0, 0" "3.000000,3.000000,3.000000")
      (Audio|PlaySoundatLocation "/Game/StarterContent/Audio/Explosion_Cue.Explosion_Cue" InputPin "0, 0, 0" 0.1 1.0 0.0 0 0 0 0)
      (Audio|PlaySoundatLocation "/Game/Assets/Sound/MolotofSound.MolotofSound" InputPin "0, 0, 0" 1.0 1.0 0.0 0 0 0 0)
      (Audio|PlaySoundatLocation "/Game/Assets/Sound/MolotofFireLand.MolotofFireLand" InputPin (Math|Conversions|RotationFromXVector InputPin) 1.0 1.0 0.0 0 0 0 0)
      (bind _returnvalue (Niagara|SpawnSystematLocation "/Game/Fire/Niagara/Fire/NFire_00.NFire_00" (Math|Vector|MakeVector _x _y 0.0) (Math|Conversions|RotationFromXVector InputPin) "2.500000,1.500000,1.600000"))
      (bind _output_get (Variables|Default|SetFireLand _returnvalue))
      (Rendering|Decal|SpawnDecalatLocation "/Game/Assets/Ickiler/M_Decal.M_Decal" "100.000000,100.000000,100.000000" (Math|Vector|MakeVector _x_2 _y_2 0.0) "-90.000000,0.000000,0.000000" 7.0)
      (Camera|PlayWorldCameraShake "/Game/Blueprints/CameraShake/BP_CamSHakee.BP_CamSHakee_C" InputPin 0.0 1.25e+04)
      (return InputPin _output_get))))