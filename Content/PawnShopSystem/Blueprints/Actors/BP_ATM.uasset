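; BP_ATM is the interactable ATM actor in the pawn shop system, opening the W_ATM screen when the player uses it.
; Its Box overlap enables input, shows the W_Interact prompt and opens a Gate, all reversed when the player leaves.
; Pressing Interact through the open Gate disables character movement, clears the GameInstance's AllowCameraTurn flag and adds a new ATM widget to the viewport.
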(event OnComponentBeginOverlap(Box)
  (params (OverlappedComponent :type Primitive%20Component%20Object%20Reference) (OtherActor :type Actor%20Object%20Reference) (OtherComp :type Primitive%20Component%20Object%20Reference) (OtherBodyIndex :type Integer) (bFromSweep :type Boolean) (SweepResult :type Hit%20Result%20Structure%20%28by%20ref%29))
  ;[0 0 0] Enable Input on Overlaping
  (if (== OtherActor (Game|GetPlayerCharacter 0))
    (Input|EnableInput (Game|GetPlayerController 0))
    (UserInterface|Viewport|AddtoViewport (Variables|Default|GetW_Interact) 0)
    (Utilities|FlowControl|Gate true) ; enters at Open
  ))

(event OnComponentEndOverlap(Box)
  (params (OverlappedComponent :type Primitive%20Component%20Object%20Reference) (OtherActor :type Actor%20Object%20Reference) (OtherComp :type Primitive%20Component%20Object%20Reference) (OtherBodyIndex :type Integer))
  ;[0 0 0] Enable Input on Overlaping
  (if (== (Game|GetPlayerCharacter 0) OtherActor)
    (Input|DisableInput (Game|GetPlayerController 0))
    (Widget|RemovefromParent (Variables|Default|GetW_Interact))
    (Utilities|FlowControl|Gate true) ; enters at Close
  ))

(event EventBeginPlay
  (bind _returnvalue (UserInterface|CreateWidget "/Game/PawnShopSystem/Widgets/W_Interact.W_Interact_C" 0 (Variables|Default|GetInteraction%20Name)))
  (Variables|Default|SetW_Interact _returnvalue))

(event Input|ActionEvents|InputActionInteract
  (params (Key :type Key%20Structure :default "None"))
  ;[0 0 0] Enable Input on Overlaping
  (:Pressed
    (Utilities|FlowControl|Gate true
      (:Exit
        ;[0 0 0] Disable player movement and prevent camera to turn
        (Pawn|Components|CharacterMovement|SetMovementMode (Variables|/Script/Engine.Character|GetCharacterMovement (Game|GetPlayerCharacter 0)) "MOVE_None" 0)
        (Variables|/Game/PawnShopSystem/Blueprints/Classes/BP_GameInstance.BP_GameInstance_C|SetAllow%20Camera%20Turn (CallFunction|GetGameInstance) false)
        ;[0 0 0] Create and add widget to viewport
        (bind _returnvalue (UserInterface|CreateWidget "/Game/PawnShopSystem/Widgets/W_ATM.W_ATM_C"))
        (UserInterface|Viewport|AddtoViewport _returnvalue 0)))))

(fn ConstructionScript)