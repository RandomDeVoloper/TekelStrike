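; BP_Shopkeeper is an interactable shop NPC actor that opens the pawn shop menu.
; Overlapping its Box enables input and shows an interaction prompt; leaving hides it and resets the interaction.
; A Gate limits the Interact action to that overlap, and a DoOnce allows one opening per visit.
; Interacting removes the prompt, stops player movement, copies the shopkeeper's items to the GameInstance, then displays W_PawnshopMenu.
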(event OnComponentBeginOverlap(Box)
  (params (OverlappedComponent :type Primitive%20Component%20Object%20Reference) (OtherActor :type Actor%20Object%20Reference) (OtherComp :type Primitive%20Component%20Object%20Reference) (OtherBodyIndex :type Integer) (bFromSweep :type Boolean) (SweepResult :type Hit%20Result%20Structure%20%28by%20ref%29))
  (bind _returnvalue (Game|GetPlayerCharacter 0))
  (bind _w_interact (Variables|Default|GetW_Interact))
  ;[0 0 0] Player interaction
  (if (== OtherActor _returnvalue)
    (Input|EnableInput (Game|GetPlayerController 0))
    (UserInterface|Viewport|AddtoViewport _w_interact 0)
    (Utilities|FlowControl|Gate true) ; enters at Open
  ))

(event OnComponentEndOverlap(Box)
  (params (OverlappedComponent :type Primitive%20Component%20Object%20Reference) (OtherActor :type Actor%20Object%20Reference) (OtherComp :type Primitive%20Component%20Object%20Reference) (OtherBodyIndex :type Integer))
  (bind _returnvalue (Game|GetPlayerCharacter 0))
  (bind _w_interact (Variables|Default|GetW_Interact))
  ;[0 0 0] Player interaction
  (if (== _returnvalue OtherActor)
    (Input|DisableInput (Game|GetPlayerController 0))
    (Widget|RemovefromParent _w_interact)
    (Utilities|FlowControl|Sequence
      (:then_0
        (Utilities|FlowControl|Gate true) ; enters at Close
      )
      (:then_1
        ;[0 0 0] remove interaction widget from viewport and stop player movement
        (Utilities|FlowControl|DoOnce false) ; enters at Reset
      ))))

(event EventBeginPlay
  ;[0 0 0] Create interaction widget reference
  (bind _returnvalue (UserInterface|CreateWidget "/Game/PawnShopSystem/Widgets/W_Interact.W_Interact_C" 0 (Variables|Default|GetInteraction%20Name)))
  (Variables|Default|SetW_Interact _returnvalue))

(event Input|ActionEvents|InputActionInteract
  (params (Key :type Key%20Structure :default "None"))
  ;[0 0 0] Player interaction
  (:Pressed
    (Utilities|FlowControl|Gate true
      (:Exit
        ;[0 0 0] remove interaction widget from viewport and stop player movement
        (Utilities|FlowControl|DoOnce false
          (:Completed
            (Widget|RemovefromParent (Variables|Default|GetW_Interact))
            (Pawn|Components|CharacterMovement|SetMovementMode (Variables|/Script/Engine.Character|GetCharacterMovement (Game|GetPlayerCharacter 0)) "MOVE_None" 0)
            ;[0 0 0] Add created items to item structure to be purchasable in the menu
            (Variables|/Game/PawnShopSystem/Blueprints/Classes/BP_GameInstance.BP_GameInstance_C|SetS_Items (CallFunction|GetGameInstance) (Variables|Default|GetS_Items))
            ;[0 0 0] Add widget to viewport
            (bind _returnvalue (UserInterface|CreateWidget "/Game/PawnShopSystem/Widgets/W_PawnshopMenu.W_PawnshopMenu_C"))
            (UserInterface|Viewport|AddtoViewport _returnvalue 0)))))))

(fn ConstructionScript)