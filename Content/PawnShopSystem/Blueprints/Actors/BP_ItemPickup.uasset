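; Pickup actor for the pawn shop system that adds its item, with quantity and pricing, to the player's inventory and destroys itself.
; Box overlap enables input, shows the W_Interact prompt and opens a Gate for the Interact action; leaving reverses this.
; The mesh's first hit triggers a delayed explosion, then randomly plays a voice clip or destroys the actor and leaves a decal.
; Debug prints accompany mesh overlaps and hits.
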(event OnComponentBeginOverlap(Box)
  (params (OverlappedComponent :type Primitive%20Component%20Object%20Reference) (OtherActor :type Actor%20Object%20Reference) (OtherComp :type Primitive%20Component%20Object%20Reference) (OtherBodyIndex :type Integer) (bFromSweep :type Boolean) (SweepResult :type Hit%20Result%20Structure%20%28by%20ref%29))
  ;[0 0 0] Player Interaction
  (if (== OtherActor (Game|GetPlayerCharacter 0))
    (Input|EnableInput (Game|GetPlayerController 0))
    (bind _returnvalue (UserInterface|CreateWidget "/Game/PawnShopSystem/Widgets/W_Interact.W_Interact_C" 0 (Variables|Default|GetInteraction%20Name)))
    (UserInterface|Viewport|AddtoViewport _returnvalue 0)
    (Utilities|FlowControl|Gate true) ; enters at Open
  ))

(event OnComponentEndOverlap(Box)
  (params (OverlappedComponent :type Primitive%20Component%20Object%20Reference) (OtherActor :type Actor%20Object%20Reference) (OtherComp :type Primitive%20Component%20Object%20Reference) (OtherBodyIndex :type Integer))
  ;[0 0 0] Player Interaction
  (if (== (Game|GetPlayerCharacter 0) OtherActor)
    (Input|DisableInput (Game|GetPlayerController 0))
    (Widget|RemovefromParent (stale OnComponentBeginOverlap(Box) _returnvalue))
    (Utilities|FlowControl|Gate true) ; enters at Close
  ))

(event OnComponentBeginOverlap(StaticMesh)
  (params (OverlappedComponent :type Primitive%20Component%20Object%20Reference) (OtherActor :type Actor%20Object%20Reference) (OtherComp :type Primitive%20Component%20Object%20Reference) (OtherBodyIndex :type Integer) (bFromSweep :type Boolean) (SweepResult :type Hit%20Result%20Structure%20%28by%20ref%29))
  (bind _asbp_player_character (Utilities|Casting|CastToBP_PlayerCharacter OtherActor))
  (Development|PrintString (Utilities|GetDisplayName _asbp_player_character)))

(event OnComponentHit(StaticMesh)
  (params (HitComponent :type Primitive%20Component%20Object%20Reference) (OtherActor :type Actor%20Object%20Reference) (OtherComp :type Primitive%20Component%20Object%20Reference) (NormalImpulse :type Vector :default "0, 0, 0") (Hit :type Hit%20Result%20Structure%20%28by%20ref%29))
  (bind _returnvalue (Math|Random|RandomIntegerinRange 0 10))
  (bind _returnvalue_2 (>= _returnvalue 5))
  (Utilities|FlowControl|DoOnce false
    (:Completed
      (Utilities|FlowControl|Delay 1.0)
      (Development|PrintString "AAAAGHHHH KAFAAAAM" true true "(R=1.000000,G=0.000000,B=0.104523,A=1.000000)")
      (Effects|SpawnEmitteratLocation "/Game/StarterContent/Particles/P_Explosion.P_Explosion" (.location Hit))
      (Audio|PlaySoundatLocation "/Game/StarterContent/Audio/Explosion01.Explosion01" (.location Hit) "0, 0, 0" 1.0 1.0 0.0 0 0 0 0)
      (Development|PrintString (Utilities|String|ToString(Boolean) _returnvalue_2))
      (if _returnvalue_2
        (Audio|PlaySound2D "/Game/Ulan-Gerizekalı-Nereye-Atıyorsun-Ses-Efekti-_uCWYe0-FLS8_.Ulan-Gerizekalı-Nereye-Atıyorsun-Ses-Efekti-_uCWYe0-FLS8_" 1.0 1.0 0.0 0 0)
        (else
          (Development|PrintString "tuttu")
          (Actor|DestroyActor)
          (Rendering|Decal|SpawnDecalatLocation "/Game/M_Decal.M_Decal" "100.000000,100.000000,100.000000" (.location Hit) "-90.000000,0.000000,0.000000" 1e+01))))))

(event Input|ActionEvents|InputActionInteract
  (params (Key :type Key%20Structure :default "None"))
  ;[0 0 0] Player Interaction
  (:Pressed
    (Utilities|FlowControl|Gate true
      (:Exit
        ;[0 0 0] Add item to player inventory and destroy actor after pickup
        (CallFunction|AddItemtoInventory (Variables|Default|GetItem%20Name) (Variables|Default|GetQuantity) (Variables|Default|GetRetail%20Price) (Variables|Default|GetMinimal%20Offer))
        (Actor|DestroyActor)))))

(fn ConstructionScript)