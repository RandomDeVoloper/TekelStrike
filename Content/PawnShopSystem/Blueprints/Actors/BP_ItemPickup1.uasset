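; BP_ItemPickup1 is a pawn shop item pickup that the player collects with the Interact input.
; Its box overlap enables input, shows a W_Interact prompt and opens a gate for the player character, and end overlap reverses this.
; Pressing Interact while the gate is open removes the prompt, adds the item with its name, quantity, retail price and minimal offer to the inventory, then destroys the actor.
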(event OnComponentBeginOverlap(Box)
  (params (OverlappedComponent :type Primitive%20Component%20Object%20Reference) (OtherActor :type Actor%20Object%20Reference) (OtherComp :type Primitive%20Component%20Object%20Reference) (OtherBodyIndex :type Integer) (bFromSweep :type Boolean) (SweepResult :type Hit%20Result%20Structure%20%28by%20ref%29))
  ;[0 0 0] Player Interaction
  (if (== OtherActor (Game|GetPlayerCharacter 0))
    (Input|EnableInput (Game|GetPlayerController 0))
    (bind _returnvalue (UserInterface|CreateWidget "/Game/PawnShopSystem/Widgets/W_Interact.W_Interact_C" 0 (Variables|Default|GetInteraction%20Name)))
    (UserInterface|Viewport|AddtoViewport _returnvalue 0)
    (Utilities|FlowControl|Gate true) ; enters at Open
  ))

(event OnComponentEndOverlap(Box)
  (params (OverlappedComponent :type Primitive%20Component%20Object%20Reference) (OtherActor :type Actor%20Object%20Reference) (OtherComp :type Primitive%20Component%20Object%20Reference) (OtherBodyIndex :type Integer))
  ;[0 0 0] Player Interaction
  (if (== (Game|GetPlayerCharacter 0) OtherActor)
    (Input|DisableInput (Game|GetPlayerController 0))
    (Widget|RemovefromParent (stale OnComponentBeginOverlap(Box) _returnvalue))
    (Utilities|FlowControl|Gate true) ; enters at Close
  ))

(event OnComponentHit(StaticMesh)
  (params (HitComponent :type Primitive%20Component%20Object%20Reference) (OtherActor :type Actor%20Object%20Reference) (OtherComp :type Primitive%20Component%20Object%20Reference) (NormalImpulse :type Vector :default "0, 0, 0") (Hit :type Hit%20Result%20Structure%20%28by%20ref%29)))

(event Input|ActionEvents|InputActionInteract
  (params (Key :type Key%20Structure :default "None"))
  ;[0 0 0] Player Interaction
  (:Pressed
    (Utilities|FlowControl|Gate true
      (:Exit
        (Widget|RemovefromParent (stale OnComponentBeginOverlap(Box) _returnvalue))
        ;[0 0 0] Add item to player inventory and destroy actor after pickup
        (CallFunction|AddItemtoInventory (Variables|Default|GetItem%20Name) (Variables|Default|GetQuantity) (Variables|Default|GetRetail%20Price) (Variables|Default|GetMinimal%20Offer))
        (Actor|DestroyActor)))))

(fn ConstructionScript)