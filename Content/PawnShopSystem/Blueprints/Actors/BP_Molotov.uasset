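; BP_Molotov is a molotov item that can be picked up into the player's inventory or explode after landing.
; A Box overlap gates the interact prompt and input for pickup.
; The mesh records its last hit location and, on physics sleep, either randomly spawns explosion, fire, decal and sounds before destroying itself, or plays a voice clip and police popup.
; High landings always take the failure branch; no damage is applied.
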(event OnComponentBeginOverlap(Box)
  (params (OverlappedComponent :type Primitive%20Component%20Object%20Reference) (OtherActor :type Actor%20Object%20Reference) (OtherComp :type Primitive%20Component%20Object%20Reference) (OtherBodyIndex :type Integer) (bFromSweep :type Boolean) (SweepResult :type Hit%20Result%20Structure%20%28by%20ref%29))
  ;[0 0 0] Player Interaction
  (if (== OtherActor (Game|GetPlayerCharacter 0))
    (Input|EnableInput (Game|GetPlayerController 0))
    (bind _returnvalue (UserInterface|CreateWidget "/Game/PawnShopSystem/Widgets/W_Interact.W_Interact_C" 0 (Variables|Default|GetInteraction%20Name)))
    (UserInterface|Viewport|AddtoViewport _returnvalue 0)
    (Utilities|FlowControl|Gate true) ; enters at Open
  ))

(event OnComponentEndOverlap(Box)
  (params (OverlappedComponent :type Primitive%20Component%20Object%20Reference) (OtherActor :type Actor%20Object%20Reference) (OtherComp :type Primitive%20Component%20Object%20Reference) (OtherBodyIndex :type Integer))
  ;[0 0 0] Player Interaction
  (if (== (Game|GetPlayerCharacter 0) OtherActor)
    (Input|DisableInput (Game|GetPlayerController 0))
    (Widget|RemovefromParent (stale OnComponentBeginOverlap(Box) _returnvalue))
    (Utilities|FlowControl|Gate true) ; enters at Close
  ))

(event OnComponentBeginOverlap(StaticMesh)
  (params (OverlappedComponent :type Primitive%20Component%20Object%20Reference) (OtherActor :type Actor%20Object%20Reference) (OtherComp :type Primitive%20Component%20Object%20Reference) (OtherBodyIndex :type Integer) (bFromSweep :type Boolean) (SweepResult :type Hit%20Result%20Structure%20%28by%20ref%29))
  (bind _asbp_player_character (Utilities|Casting|CastToBP_PlayerCharacter OtherActor))
  (Development|PrintString (Utilities|GetDisplayName _asbp_player_character)))

(event OnComponentHit(StaticMesh)
  (params (HitComponent :type Primitive%20Component%20Object%20Reference) (OtherActor :type Actor%20Object%20Reference) (OtherComp :type Primitive%20Component%20Object%20Reference) (NormalImpulse :type Vector :default "0, 0, 0") (Hit :type Hit%20Result%20Structure%20%28by%20ref%29))
  (bind _output_get (Variables|Default|SetHit%20Location (.location Hit))))

(event OnComponentSleep(StaticMesh)
  (params (SleepingComponent :type Primitive%20Component%20Object%20Reference) (BoneName :type Name :default "None"))
  (Utilities|FlowControl|DoOnce false
    (:Completed
      (Development|PrintString (Utilities|String|ToString(Vector) (stale OnComponentHit(StaticMesh) _output_get)) true true "(R=1.000000,G=0.573996,B=0.000000,A=1.000000)")
      (if (>= (.Z (Math|Vector|BreakVector (stale OnComponentHit(StaticMesh) _output_get))) 1e+02)
        ;[0.15 0.15 0.15 0.5] ULAN GERİZEKALI NEREYE ATIYOSUN
        (Audio|PlaySound2D "/Game/Developers/Ulan-Gerizekalı-Nereye-Atıyorsun-Ses-Efekti-_uCWYe0-FLS8_.Ulan-Gerizekalı-Nereye-Atıyorsun-Ses-Efekti-_uCWYe0-FLS8_" 2.0 1.0 0.0 0 0 :!label _label)
        ;[0.15 0.15 0.15 0.5] POLİS WİDGETI
        (Utilities|FlowControl|DoOnce false :!label _label_2
          (:Completed
            (Utilities|FlowControl|Delay 0.04)
            (bind _returnvalue (UserInterface|CreateWidget "/Game/Widgets/WBP_Polis.WBP_Polis_C" (Game|GetPlayerController 0)))
            (bind _output_get (Variables|Default|SetWBP_PolicREF _returnvalue))
            (UserInterface|Viewport|AddtoViewport _output_get 0)
            (UserInterface|Animation|PlayAnimation _output_get (Variables|/Game/Widgets/WBP_Polis.WBP_Polis_C|GetPopUpAnim _output_get) 0.0 1 "Forward" 0.7 false)
            (Utilities|FlowControl|Delay 1.5)
            (Widget|RemovefromParent (Variables|Default|GetWBP_PolicREF))
            (goto _label_2 Reset)))
        (elif (>= (Math|Random|RandomIntegerinRange 0 10) 5)
          (Utilities|FlowControl|Delay 0.3)
          ;[0.15 0.15 0.15 0.5] Bottle Broke Sound
          (Audio|PlaySoundatLocation "/Game/Assets/Sound/MolotofSound.MolotofSound" (stale OnComponentHit(StaticMesh) _output_get) "0, 0, 0" 1.0 1.0 0.0 0 0 0 0)
          ;[0.15 0.008488 0 0.5] BOMBA PATLAMA (Hasar sistemi + ragdoll + mimarilerde hasar yıkım. )
          (Effects|SpawnEmitteratLocation "/Game/StarterContent/Particles/P_Explosion.P_Explosion" (stale OnComponentHit(StaticMesh) _output_get) "0, 0, 0" "3.000000,3.000000,3.000000")
          (Audio|PlaySoundatLocation "/Game/StarterContent/Audio/Explosion01.Explosion01" (stale OnComponentHit(StaticMesh) _output_get) "0, 0, 0" 1.0 1.0 0.0 0 0 0 0)
          (Development|PrintString "tuttu")
          (Actor|DestroyActor)
          (Audio|PlaySoundatLocation "/Game/Assets/Sound/MolotofFireLand.MolotofFireLand" (stale OnComponentHit(StaticMesh) _output_get) "0, 0, 0" 1.0 1.0 0.0 0 0 0 0)
          (bind _returnvalue_2 (Effects|SpawnEmitteratLocation "/Game/Fire/Particles/Fire/Fire_00.Fire_00" (stale OnComponentHit(StaticMesh) _output_get) "0, 0, 0" "3.000000,2.000000,1.000000" true "AutoRelease"))
          (Rendering|Decal|SpawnDecalatLocation "/Game/Assets/M_Decal.M_Decal" "100.000000,100.000000,100.000000" (stale OnComponentHit(StaticMesh) _output_get) "-90.000000,0.000000,0.000000" 1e+01)
          (Utilities|FlowControl|Delay 3.0)
          (Components|DestroyComponent _returnvalue_2)
          (else
            (goto _label)))))))

(event Input|ActionEvents|InputActionInteract
  (params (Key :type Key%20Structure :default "None"))
  ;[0 0 0] Player Interaction
  (:Pressed
    (Utilities|FlowControl|Gate true
      (:Exit
        ;[0 0 0] Add item to player inventory and destroy actor after pickup
        (CallFunction|AddItemtoInventory (Variables|Default|GetItem%20Name) (Variables|Default|GetQuantity) (Variables|Default|GetRetail%20Price) (Variables|Default|GetMinimal%20Offer))
        (Actor|DestroyActor)))))

(fn ConstructionScript)