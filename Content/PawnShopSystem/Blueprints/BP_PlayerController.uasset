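; Player controller for the pawn shop system that tracks whether the player is using a gamepad or mouse and keyboard.
; Any key press sets the UsingGamepad flag on the game instance according to whether the key is a gamepad key.
; Mouse axis movement above a small threshold clears the flag, though the duplicated check only catches movement in the positive direction.
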(event Input|MouseEvents|MouseY
  (params (AxisValue :type Float%20%28single-precision%29))
  ;[0 0 0] Check is Mouse is in Use
  (if (or (> (stale Input|MouseEvents|MouseX AxisValue) 0.1) (> AxisValue 0.1))
    (Variables|/Game/PawnShopSystem/Blueprints/Classes/BP_GameInstance.BP_GameInstance_C|SetUsing%20Gamepad? (CallFunction|GetGameInstance) false)))

(event Input|MouseEvents|MouseX
  (params (AxisValue :type Float%20%28single-precision%29))
  ;[0 0 0] Check is Mouse is in Use
  (if (or (> AxisValue 0.1) (> (stale Input|MouseEvents|MouseY AxisValue) 0.1))
    (Variables|/Game/PawnShopSystem/Blueprints/Classes/BP_GameInstance.BP_GameInstance_C|SetUsing%20Gamepad? (CallFunction|GetGameInstance) false)))

(event Input|KeyboardEvents|AnyKey
  (params (Key :type Key%20Structure :default "None"))
  (bind _return_value (CallFunction|GetGameInstance))
  ;[0 0 0] Check if Input is Gamepad Key
  (:Pressed
    (if (Class|KismetInputLibrary|KeyIsGamepadKey Key)
      (Variables|/Game/PawnShopSystem/Blueprints/Classes/BP_GameInstance.BP_GameInstance_C|SetUsing%20Gamepad? _return_value true)
      (else
        (Variables|/Game/PawnShopSystem/Blueprints/Classes/BP_GameInstance.BP_GameInstance_C|SetUsing%20Gamepad? _return_value false)))))

(fn ConstructionScript)