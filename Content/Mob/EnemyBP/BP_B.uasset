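; BP_B is an enemy Blueprint with a health-bar widget update and a kick-death macro.
; At zero health, OnKickedMacro turns the mesh into a ragdoll launched by a pelvis impulse, with a kick sound and a timed IsDeadly window.
; It then awards the player XP, spawns a BP_Soul and destroys the enemy.
; Capsule overlap only prints the player's name, and WalkAnim is empty.
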(event OnComponentBeginOverlap(CapsuleComponent)
  (params (OverlappedComponent :type Primitive%20Component%20Object%20Reference) (OtherActor :type Actor%20Object%20Reference) (OtherComp :type Primitive%20Component%20Object%20Reference) (OtherBodyIndex :type Integer) (bFromSweep :type Boolean) (SweepResult :type Hit%20Result%20Structure%20%28by%20ref%29))
  (bind _asbp_player_character (Utilities|Casting|CastToBP_PlayerCharacter OtherActor))
  (Development|PrintString (Utilities|GetDisplayName _asbp_player_character)))

(fn ConstructionScript)

(fn HealthBar
  (params (CurrentHealth :type Float%20%28single-precision%29) (MaxHealth :type Float%20%28double-precision%29))
  (bind _aswbp_hp_hud (Utilities|Casting|CastToWBP_HpHUD (UserInterface|GetUserWidgetObject (Variables|Default|GetHealthBarW))))
  (Default|UpdateHealBar _aswbp_hp_hud CurrentHealth MaxHealth))

(fn WalkAnim
  (params (Enemy :type Actor%20Object%20Reference))
  (return 0 0))