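; BP_C2 is an enemy that can be kicked away as a ragdoll once its health reaches zero.
; The kick macro enables mesh physics, plays a randomized sound, applies a pelvis impulse and keeps IsDeadly set during the bounce.
; It then awards player XP and, after a delay, spawns a BP_Soul and destroys itself.
; A Molotov hit destroys it directly; HealthBar and WalkAnim are effectively empty.
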(event Custom|MolotofIsabet
  (Actor|DestroyActor)
  (Components|DestroyComponent (Variables|Collision|GetCapsuleComponent self)))

(fn ConstructionScript)

(fn HealthBar
  (params (CurrentHealth :type Float%20%28single-precision%29) (MaxHealth :type Float%20%28double-precision%29)))

(fn WalkAnim
  (params (Enemy :type Actor%20Object%20Reference))
  (return 0 0))