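; BP_SpawnB is a self-limiting spawner actor that creates BP_B pawns running BT_Enemy at its own location and rotation.
; BeginPlay spawns one immediately, then starts a looping timer whose interval is fixed at the initial Duration.
; Each spawn decrements Duration, which acts as a countdown without retiming the timer, and the actor destroys itself once it reaches zero.
; The AISpawner function is empty.
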(event Custom|AISPAWN
  (AI|SpawnAIFromClass "/Game/Mob/EnemyBP/BP_B.BP_B_C" "/Game/Mob/AI/BeheviorTree/BT_Enemy.BT_Enemy" (Transformation|GetActorLocation self) (Transformation|GetActorRotation) false 0)
  (bind _output_get (Variables|Default|SetDuration (- (Variables|Default|GetDuration) 0.1)))
  (if (<= _output_get 0.0)
    (Actor|DestroyActor)))

(event EventBeginPlay
  (CallFunction|AISPAWN)
  (Utilities|Time|SetTimerbyEvent (delegate Custom|AISPAWN) (Variables|Default|GetDuration) true))

(fn ConstructionScript)

(fn AISpawner)