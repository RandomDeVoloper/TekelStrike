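; BP_SpawnC is an enemy spawner that creates BP_C pawns running the BT_Enemy behavior tree at its own location and rotation.
; It spawns once on BeginPlay, then repeats on a looping timer whose interval is the initial Duration.
; Each spawn lowers Duration and prints it, but the timer is never reset and the zero check does nothing.
; The construction script and AISpawner function are empty.
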(event Custom|AISPAWN
  (AI|SpawnAIFromClass "/Game/Mob/EnemyBP/BP_C.BP_C_C" "/Game/Mob/AI/BeheviorTree/BT_Enemy.BT_Enemy" (Transformation|GetActorLocation self) (Transformation|GetActorRotation) false 0)
  (bind _output_get (Variables|Default|SetDuration (- (Variables|Default|GetDuration) 0.1)))
  (Development|PrintString (Utilities|String|ToString(Float) _output_get))
  (if (<= _output_get 0.0)
    _))

(event EventBeginPlay
  (CallFunction|AISPAWN)
  (Utilities|Time|SetTimerbyEvent (delegate Custom|AISPAWN) (Variables|Default|GetDuration) true))

(fn ConstructionScript)

(fn AISpawner)